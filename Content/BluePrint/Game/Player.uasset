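; Player Blueprint that detects touch swipes and prints their direction as Left, Right, Up or Down.
; Touch press and release record screen positions, and Tick calls a swipe check once a touch has occurred.
; When start-to-end distance passes a threshold, a DoOnce, reset on release, re-reads the touch position and picks the direction from the dominant axis.
; The touched flag is never cleared, and directions only print, with no movement attached.
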(event `self.ReceiveTick`
  (params (DeltaSeconds :type "Float (single-precision)"))
  (if (`self.Is Touched`)
    (`self.Check_Swiping`)))

(event `InputTouch`
  (params (Location :type "Vector Structure") (FingerIndex :type "ETouchIndex Enum"))
  (bind _x (.x Location))
  (bind _y (.y Location))
  (bind (_locationx _locationy) (`PlayerController.GetInputTouchState` (`GameplayStatics.GetPlayerController` 0) "Touch1"))
  (bind (_x_2 _y_2) (`KismetMathLibrary.BreakVector2D` (- (`self.Touch Start`) (`self.Touch End`))))
  (:`Pressed`
    (set `self.Is Touched` true)
    (set `self.Touch Start` (`KismetMathLibrary.MakeVector2D` _x _y)))
  (:`Released`
    (set `self.Touch End` (`KismetMathLibrary.MakeVector2D` _x _y))
    (goto _label :!via `Reset`)))

(event `Check_Swiping`
  (bind (_locationx _locationy) (`PlayerController.GetInputTouchState` (`GameplayStatics.GetPlayerController` 0) "Touch1"))
  (bind (_x _y) (`KismetMathLibrary.BreakVector2D` (- (`self.Touch Start`) (`self.Touch End`))))
  (if (> (`KismetMathLibrary.VSize2D` (- (`self.Touch Start`) (`self.Touch End`))) 100.0)
    (`/Engine/EditorBlueprintResources/StandardMacros.DoOnce` false :!label _label
      (:`Completed`
        (set `self.Touch End` (`KismetMathLibrary.MakeVector2D` _locationx _locationy))
        (if (> (`KismetMathLibrary.Abs` _x) (`KismetMathLibrary.Abs` _y))
          (if (> _x 0.0)
            (`KismetSystemLibrary.PrintString` "Left")
            (else
              (`KismetSystemLibrary.PrintString` "Right")))
          (elif (> _y 0.0)
            (`KismetSystemLibrary.PrintString` "Up")
            (else
              (`KismetSystemLibrary.PrintString` "Down"))))))))

(fn `UserConstructionScript`)